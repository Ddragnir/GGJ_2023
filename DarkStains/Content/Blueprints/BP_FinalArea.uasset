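; BP_FinalArea is an actor that holds the game's ending sequence.
; Its CineEnd event takes the player, hides their HUD bars and level display, fades the camera out, disables input, then plays final audio and shows the WG_Final widget.
; After a timed delay it opens GameMap.
; The overlap event only casts to BP_Player, and nothing in this graph calls CineEnd.
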(event `self.ReceiveActorBeginOverlap`
  (params (OtherActor :type "Actor Object Reference"))
  (cast `/Game/Blueprints/BP_Player` OtherActor))

(event `CineEnd`
  (params (Player :type "/Game/Blueprints/BP_Player Object Reference"))
  (`/Game/Blueprints/Widgets/BP_StaminaWidget.ShowStamina` (`/Game/Blueprints/BP_Player.StaminaBar` Player) false)
  (`Widget.SetVisibility` (`/Game/Blueprints/BP_Player.PlayerBars` Player) "Hidden")
  (`Widget.SetVisibility` (`/Game/Blueprints/BP_Player.PlayerLvl` Player) "Hidden")
  (`PlayerCameraManager.StartCameraFade` :`self` (`GameplayStatics.GetPlayerCameraManager` 0) :`ToAlpha` 1.0 :`Duration` 2.0 :`bHoldWhenFinished` true)
  (`KismetSystemLibrary.Delay` 2.0)
  (`self.DisableInput` Player (`GameplayStatics.GetPlayerController` 0))
  (`GameplayStatics.SpawnSound2D` "/Game/Audio/Music/MSC_Final.MSC_Final" 1.0 1.0 0.0 null)
  (bind _returnvalue (`|CreateWidget` "/Game/Blueprints/Widgets/WG_Final.WG_Final_C" (`GameplayStatics.GetPlayerController` 0)))
  (`UserWidget.AddToPlayerScreen` _returnvalue 0)
  (`KismetSystemLibrary.Delay` 10.0)
  (`GameplayStatics.OpenLevel` "GameMap"))

(fn `UserConstructionScript`)