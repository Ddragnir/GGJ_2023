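; BP_CameraMenu is the main menu camera actor, which shows the WG_Menu widget and handles the handoff to gameplay.
; D-pad up/down or Enter hides the cursor and gives the Start button keyboard focus.
; Starting masks a timed view blend to BP_Player with its ink screen, plays BP_BossDoor's zone music, then possesses and initializes the player; quitting exits.
; An unconnected level-sequence intro remains unused.
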(event `self.ReceiveBeginPlay`
  (bind _returnvalue (`GameplayStatics.GetPlayerController` 0))
  (set `PlayerController.bShowMouseCursor` true _returnvalue)
  (bind _returnvalue_2 (`|CreateWidget` "/Game/Blueprints/Widgets/WG_Menu.WG_Menu_C" _returnvalue))
  (bind _output_get (set `self.WGMenu` _returnvalue_2))
  (`UserWidget.AddToViewport` _output_get 0)
  (bind _returnvalue_3 (`GameplayStatics.GetActorOfClass` "/Game/Blueprints/BP_BossDoor.BP_BossDoor_C"))
  (set `self.BossDoor` _returnvalue_3))

(event `Key|Gamepad_DPad_Up`
  (params (Key :type "Key Structure"))
  (bind _returnvalue (`GameplayStatics.GetPlayerController` 0))
  (:`Pressed`
    (`WidgetBlueprintLibrary.SetInputMode_GameAndUIEx` _returnvalue (stale `self.ReceiveBeginPlay` _output_get) :!label _label)
    (set `PlayerController.bShowMouseCursor` false _returnvalue)
    (`KismetSystemLibrary.Delay` 0.1)
    (`Widget.SetKeyboardFocus` (`/Game/Blueprints/Widgets/WG_Menu.Start` (stale `self.ReceiveBeginPlay` _output_get)))
    (`KismetSystemLibrary.PrintString` "Hello")))

(event `Key|Enter`
  (params (Key :type "Key Structure"))
  (:`Pressed`
    (goto _label)))

(event `Key|Gamepad_DPad_Down`
  (params (Key :type "Key Structure"))
  (:`Pressed`
    (goto _label)))

(event `CommencerButton Pressed`
  (bind _returnvalue (`GameplayStatics.GetPlayerController` 0))
  (bind _returnvalue_2 (`GameplayStatics.GetActorOfClass` "/Game/Blueprints/BP_Player.BP_Player_C"))
  (`/Game/Blueprints/BP_Player.Death Ink Screen` _returnvalue_2 false 0.0)
  (`Widget.RemoveFromParent` (`self.WGMenu`))
  (`KismetSystemLibrary.Delay` 1.0)
  (`PlayerController.SetViewTargetWithBlend` _returnvalue _returnvalue_2 2.0 "VTBlend_Cubic" 1.0 false)
  (`/Game/Blueprints/BP_BossDoor.PlayZoneMus` (`self.BossDoor`))
  (`KismetSystemLibrary.Delay` 0.5)
  (`/Game/Blueprints/BP_Player.Death Ink Screen` _returnvalue_2 true 0.0)
  (`Controller.Possess` _returnvalue _returnvalue_2)
  (`KismetSystemLibrary.Delay` 1.0)
  (`/Game/Blueprints/BP_Player.InitPlayer` _returnvalue_2))

(event `QuitterButtonPressed`
  (`KismetSystemLibrary.QuitGame` null "Quit"))

(fn `UserConstructionScript`)