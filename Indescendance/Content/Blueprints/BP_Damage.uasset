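; BP_Damage is a floating damage number actor that shows a damage value and flies off in a random direction.
; SpawnDamage writes the value into the WG_Damage widget and applies a random velocity-change impulse on all three axes to the static mesh.
; The actor destroys itself when the widget signals that its lifetime is over.
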(event `SpawnDamage`
  (params (DamageValue :type "Float (double-precision)"))
  (bind _aswg_damage (cast `/Game/Blueprints/WG_Damage` (`WidgetComponent.GetUserWidgetObject` (`self.Widget`))))
  (add `/Game/Blueprints/WG_Damage.WidgetLifeTimeOver` _aswg_damage (delegate `WidgetDead`))
  (message `/Game/Blueprints/IT_DamageValue.SetDamageValue` _aswg_damage (`KismetTextLibrary.Conv_DoubleToText` DamageValue "HalfToEven"))
  (`PrimitiveComponent.AddImpulse` (`self.StaticMesh`) (`KismetMathLibrary.MakeVector` (`KismetMathLibrary.RandomFloatInRange` -400.0 400.0) (`KismetMathLibrary.RandomFloatInRange` -400.0 400.0) (`KismetMathLibrary.RandomFloatInRange` -400.0 400.0)) "None" true))

(event `WidgetDead`
  (`self.K2_DestroyActor`))

(fn `UserConstructionScript`)