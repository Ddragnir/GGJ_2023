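; BP_BossDoorOut is a boss door actor, apparently the exit, whose OpenDoor event currently handles only the audio transition.
; On BeginPlay it caches the first BP_BossDoor found in the level.
; OpenDoor stops that door's boss music, then fades in its ambient zone sound after a short delay.
; A delayed timeline that would swing the two door pivots open is disconnected, so this door never animates.
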(event `self.ReceiveBeginPlay`
  (bind _outactors (`GameplayStatics.GetAllActorsOfClass` "/Game/Blueprints/BP_BossDoor.BP_BossDoor_C"))
  (set `self.Door` (`|GetArrayItem` _outactors)))

(event `OpenDoor`
  (bind _door (`self.Door`))
  ;[1 0 0.7079] Door Animation
  (`|ExecutionSequence`
    (:`then_1`
      (`AudioComponent.Stop` (`/Game/Blueprints/BP_BossDoor.BossMus` _door))
      (`KismetSystemLibrary.Delay` 0.5)
      (`AudioComponent.FadeIn` (`/Game/Blueprints/BP_BossDoor.SND_AmbZone` _door) 2.0 1.0 0.0 "Linear"))))

(fn `UserConstructionScript`)