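; BP_BossTotem is a short-lived boss hazard that damages the player on contact.
; On BeginPlay it waits briefly with collision off, then enables query collision and uses a sped-up timeline to lerp its root upward.
; A Cylinder overlap with BP_Player sends a DamageTarget interface message and switches collision off to stop further hits.
; When the timeline finishes, it disables collision and destroys itself after a delay.
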(event `/Game/Blueprints/IT_Damage.DamageTarget`
  (params (FromActor :type "Actor Object Reference") (FromLocation :type "Vector Structure") (DamageValue :type "Float (double-precision)") (Parable :type Boolean))
  (set `self.From Actor` FromActor)
  (set `self.From Location` FromLocation)
  (set `self.Damage Value` DamageValue)
  (set `self.Parable` Parable))

(event `EnabledCollision`
  (params (CollisionType :type "ECollisionEnabled Enum" :default "NoCollision"))
  (`PrimitiveComponent.SetCollisionEnabled` (`self.Cylinder`) CollisionType))

(event `self.ReceiveBeginPlay`
  (`self.EnabledCollision` "NoCollision")
  (`KismetSystemLibrary.Delay` 2.0)
  (`self.EnabledCollision` "QueryOnly")
  (`TimelineComponent.SetPlayRate` (`self.TM_Activation`) 3.0)
  (set `self.TotemLocation` (`SceneComponent.RelativeLocation` (`self.Root`)))
  (bind (_direction _alpha) (`Timeline|TM_Activation` :!via `PlayFromStart`)
    (:`Update`
      (`SceneComponent.K2_SetRelativeLocation` (`self.Root`) (`KismetMathLibrary.VLerp` (`self.TotemLocation`) (0.0 0.0 90.0) _alpha) false false))
    (:`Finished`
      (`self.EnabledCollision` "NoCollision")
      (`KismetSystemLibrary.Delay` 3.0)
      (`self.K2_DestroyActor`))))

(event `self.Cylinder.OnComponentBeginOverlap`
  (params (OverlappedComponent :type "PrimitiveComponent Object Reference") (OtherActor :type "Actor Object Reference") (OtherComp :type "PrimitiveComponent Object Reference") (OtherBodyIndex :type Integer) (bFromSweep :type Boolean) (SweepResult :type "HitResult Structure (by ref)"))
  (bind _asbp_player (cast `/Game/Blueprints/BP_Player` OtherActor))
  (message `/Game/Blueprints/IT_Damage.DamageTarget` _asbp_player self (`self.K2_GetActorLocation`) (`self.Damage Value`) false)
  (`self.EnabledCollision` "NoCollision"))

(fn `UserConstructionScript`)