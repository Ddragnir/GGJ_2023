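; Boss arena door that shuts behind BP_Player when they leave its detection box, starting the boss fight.
; End overlap enables the blocking collider, swaps zone audio for boss music and swings both pivots closed by timeline, then spawns BP_Boss.
; ResetDoor, meant for player death, restores zone audio and reopens the door after delays, with IsReseting preventing a respawn.
; The exit-direction check and PlayBossEntrance currently have no effect.
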(event `self.BoxDetection.OnComponentBeginOverlap`
  (params (OverlappedComponent :type "PrimitiveComponent Object Reference") (OtherActor :type "Actor Object Reference") (OtherComp :type "PrimitiveComponent Object Reference") (OtherBodyIndex :type Integer) (bFromSweep :type Boolean) (SweepResult :type "HitResult Structure (by ref)"))
  ;[1 0.4387 0] Player Enter Door Detector
  (bind _asbp_player (cast `/Game/Blueprints/BP_Player` OtherActor))
  (set `self.EnterDirection` (< (.y (`KismetMathLibrary.LessLess_VectorRotator` (- (`self.K2_GetActorLocation`) (`self.K2_GetActorLocation` _asbp_player)) (`self.K2_GetActorRotation`))) 0.0)))

(event `PlayBossEntrance`)

(event `PlayZoneMus`
  (`AudioComponent.Play` (`self.MSC_Zone`) 0.0))

(event `self.BoxDetection.OnComponentEndOverlap`
  (params (OverlappedComponent :type "PrimitiveComponent Object Reference") (OtherActor :type "Actor Object Reference") (OtherComp :type "PrimitiveComponent Object Reference") (OtherBodyIndex :type Integer))
  (bind (_returnvalue_location _returnvalue_rotation) (`KismetMathLibrary.BreakTransform` (`self.GetTransform` (`self.SpawnBoss`))))
  ;[0.1214 1 0.02871] Player Out Door Detector
  (bind _asbp_player (cast `/Game/Blueprints/BP_Player` OtherActor))
  ;;[0 0.3578 1] Check if Player Go Out Opposit Enter Direction
  (if (== (`self.EnterDirection`) (< (.y (`KismetMathLibrary.LessLess_VectorRotator` (- (`self.K2_GetActorLocation`) (`self.K2_GetActorLocation` _asbp_player)) (`self.K2_GetActorRotation`))) 0.0))
    _
    (else
      _))
  (if (>= (`/Game/Blueprints/BP_Player.LastSiecle` _asbp_player) 10)
    ;;[1 0.02122 0] Player Battle Boss First Time
    (`/Engine/EditorBlueprintResources/StandardMacros.DoOnce` false
      (:`Completed`
        (`self.PlayBossEntrance`))))
  ;;[0 1 0.4555] Block Player if Go Out
  (`PrimitiveComponent.SetCollisionEnabled` (`self.BoxCollider`) "QueryAndPhysics")
  (bind _returnvalue (`GameplayStatics.SpawnSound2D` "/Game/Audio/Music/MSC_Boss_01.MSC_Boss_01" 1.0 1.0 0.0 null))
  (set `self.BossMus` _returnvalue)
  (`AudioComponent.FadeOut` (`self.MSC_Zone`) 1.0 0.0 "Linear")
  (`AudioComponent.FadeOut` (`self.SND_AmbZone`) 1.0 0.0 "Linear")
  (set `self.isReseting` false)
  ;;[1 0 0.7079] Door Animation
  (bind (_direction _alpha) (`Timeline|TM_Door` :!via `PlayFromStart` :!label _label)
    (:`Update`
      (`SceneComponent.K2_SetRelativeRotation` (`self.RightPivot`) (`KismetMathLibrary.RLerp` (struct :`Yaw` -90.0) (struct) _alpha true) false false)
      (`SceneComponent.K2_SetRelativeRotation` (`self.LeftPivot`) (`KismetMathLibrary.RLerp` (struct :`Yaw` 90.0) (struct) _alpha true) false false))
    (:`Finished`
      (if (not (`self.isReseting`))
        ;;[0.2992 0.3709 1] Spawn Boss End Animation
        (bind _returnvalue_2 (`|SpawnActorFromClass` "/Game/Blueprints/BP_Boss.BP_Boss_C" (`KismetMathLibrary.MakeTransform` _returnvalue_location _returnvalue_rotation) "Undefined" "OverrideRootScale" null null))
        (message `/Game/Blueprints/IT_Communication.InitActor` _returnvalue_2)))))

(event `ResetDoor`
  ;[0.1214 1 0.02871] Player Out Door Detector
  ;;[1 0.4766 0] Reset Door At Player Dead
  (`/Engine/EditorBlueprintResources/StandardMacros.IsValid` (stale `self.BoxDetection.OnComponentEndOverlap` _returnvalue)
    (:`Is Valid`
      (`AudioComponent.FadeOut` (stale `self.BoxDetection.OnComponentEndOverlap` _returnvalue) 1.0 0.0 "Linear")
      (`AudioComponent.FadeIn` (`self.SND_AmbZone`) 1.0 1.0 0.0 "Linear")
      (`|ExecutionSequence`
        (:`then_0`
          (`KismetSystemLibrary.Delay` 8.0)
          (`PrimitiveComponent.SetCollisionEnabled` (`self.BoxCollider`) "NoCollision")
          (set `self.isReseting` true)
          (goto _label :!via `ReverseFromEnd`))
        (:`then_1`
          (`KismetSystemLibrary.Delay` 6.0)
          (`AudioComponent.Play` (`self.MSC_Zone`) 0.0))))))

(fn `UserConstructionScript`)