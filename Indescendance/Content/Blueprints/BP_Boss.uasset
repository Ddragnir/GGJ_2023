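; Titan boss that fights BP_Player through health phases shown on a boss bar, then opens the exit doors on death.
; A looping timer picks random attacks per phase: ground kick or wall-stopped charge, then leaping slam, hammer with pillar spawning, or projectile-spraying spin between BP_Target points.
; Montages, hit notifications, timers and timelines drive the attacks, which deal damage through sphere overlaps, capsule contact and spawned actors, with camera and VFX feedback.
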(event `PaternAction`
  (bind _paterncount (`self.PaternCount`))
  ;[1 0.04129 0] Patern
  (`KismetSystemLibrary.PrintString` (`KismetStringLibrary.Concat_StrStr` "switch patern -> " (`KismetStringLibrary.Conv_IntToString` _paterncount)))
  (switch `int` _paterncount))

(event `/Game/Blueprints/IT_Damage.DamageTarget`
  (params (FromActor :type "Actor Object Reference") (FromLocation :type "Vector Structure") (DamageValue :type "Float (double-precision)") (Parable :type Boolean))
  ;[0.2373 1 0] Enemy Take Damage
  (if (not (`self.ignoreDamage`))
    (bind _output_get (set `self.CurrentHealth` (- (`self.CurrentHealth`) DamageValue)))
    (message `/Game/Blueprints/IT_Damage.hitSuccess` FromActor)
    (`/Game/Blueprints/BP_Player.SetBossLifeBarValue` (`self.Player`) (/ _output_get (`|GetArrayItem` (`self.MaxHealth`) (`self.PaternCount`))))
    (bind _returnvalue (`|SpawnActorFromClass` "/Game/Blueprints/BP_Damage.BP_Damage_C" (`KismetMathLibrary.MakeTransform` (`self.K2_GetActorLocation`) (struct) (0.5 0.5 0.5)) "Undefined" "OverrideRootScale" null null))
    (`/Game/Blueprints/BP_Damage.SpawnDamage` _returnvalue DamageValue)
    (`NiagaraFunctionLibrary.SpawnSystemAtLocation` "/Game/VFX/_Shared/NS_Player_Hit.NS_Player_Hit" (`SceneComponent.K2_GetComponentLocation` (`self.Hit`)))
    (`NiagaraFunctionLibrary.SpawnSystemAtLocation` "/Game/VFX/_Shared/NS_Player_HitGround.NS_Player_HitGround" (`SceneComponent.K2_GetComponentLocation` (`self.Mesh`)))
    (`GameplayStatics.SpawnSound2D` "/Game/Audio/SFX/SFX_PlayerHit_Cue.SFX_PlayerHit_Cue" 1.0 1.0 0.0 null)
    (bind (_direction _emissive) (`Timeline|Emissive` :!via `PlayFromStart`)
      (:`Update`
        (`KismetMaterialLibrary.SetScalarParameterValue` "/Game/VFX/_Shared/MPC_TakesDmg.MPC_TakesDmg" "EmissiveBoss" _emissive)
        (`self.CameraShake` 0.1)
        (bind (_direction_2 _emissive_2) (`Timeline|Boss` :!via `PlayFromStart`)
          (:`Update`
            (`KismetMaterialLibrary.SetScalarParameterValue` "/Game/VFX/_Shared/MPC_TakesDmg.MPC_TakesDmg" "EmissiveBoss" _emissive_2)
            (if (<= (`self.CurrentHealth`) 0.0)
              (bind _result (`/Engine/EditorBlueprintResources/StandardMacros.IncrementInt` (`self.PaternCount`))
                (:`  `
                  (bind _output_get_2 (set `self.PaternCount` _result))
                  (`/Game/Blueprints/BP_Player.RemoveBossBar` (`self.Player`))
                  (if (> _output_get_2 (`KismetArrayLibrary.Array_Length` (`self.MaxHealth`)))
                    ;;[0.04008 0.2969 0] Death
                    (set `self.isDead` true)
                    (`KismetSystemLibrary.K2_ClearAndInvalidateTimerHandle` (`self.TimerHandler`))
                    (`KismetSystemLibrary.K2_ClearAndInvalidateTimerHandle` (`self.ToupisHandle`))
                    (`KismetSystemLibrary.K2_ClearAndInvalidateTimerHandle` (`self.PilierHandle`))
                    (set `self.isAttacking` true)
                    (set `self.ignoreDamage` true)
                    (`/Game/Blueprints/BP_Player.EncounterBoss` (`self.Player`) false 0)
                    (`TimelineComponent.Stop` (`self.TM_Spining`))
                    (bind _returnvalue_2 (`AnimInstance.PlaySlotAnimationAsDynamicMontage` (`SkeletalMeshComponent.GetAnimInstance` (`self.Mesh`)) "/Game/3d/Cha/Titan/TitanDeath.TitanDeath" "DefaultSlot" 0.25 0.25 0.7 1 -1.0 0.0))
                    ;;[0.3061 1 0.2499] Open Final Door
                    (bind _outactors (`GameplayStatics.GetAllActorsOfClass` "/Game/Blueprints/BP_BossDoorOut.BP_BossDoorOut_C"))
                    (for _array_element _outactors
                      (`/Game/Blueprints/BP_BossDoorOut.OpenDoor` _array_element))
                    (`KismetSystemLibrary.Delay` (+ (`AnimationAsset.GetPlayLength` _returnvalue_2) 1.2))
                    (`self.K2_DestroyActor`)
                    (else
                      (`self.InitHealth`))))))))))))

(event `/Game/Blueprints/IT_Communication.InitActor`
  ;[1 0 0] Enemy Attack
  (`/Game/Blueprints/BP_Player.SetBossLifeBarValue` (`self.Player`) 1.0)
  (`/Game/Blueprints/BP_Player.EncounterBoss` (`self.Player`) true (`KismetArrayLibrary.Array_Length` (`self.MaxHealth`)))
  (bind _returnvalue (`KismetSystemLibrary.K2_SetTimerDelegate` (delegate `DoAction`) 1.0 true))
  (set `self.TimerHandler` _returnvalue))

(event `self.ReceiveBeginPlay`
  ;[0.08374 0.1668 1] Begin Play
  (`|ExecutionSequence`
    (:`then_0`
      (bind _asbp_player (cast `/Game/Blueprints/BP_Player` (`GameplayStatics.GetPlayerCharacter` 0)))
      (set `self.Player` _asbp_player)
      (`self.InitHealth`)
      (`self.PlayAnimationMontage` "/Game/3d/Cha/Titan/TitanSpawn.TitanSpawn")
      (set `self.ignoreDamage` true)
      (`KismetSystemLibrary.Delay` 3.0)
      (set `self.hasspawned` true)
      (set `self.ignoreDamage` false))
    (:`then_1`
      (bind _outactors (`GameplayStatics.GetAllActorsOfClass` "/Game/Blueprints/BP_Target.BP_Target_C"))
      (set `self.targetpoint` _outactors))))

(event `InitHealth`
  (bind _output_get (set `self.CurrentHealth` (`|GetArrayItem` (`self.MaxHealth`) (`self.PaternCount`))))
  (`/Game/Blueprints/BP_Player.SetBossLifeBarValue` (`self.Player`) (/ _output_get (`|GetArrayItem` (`self.MaxHealth`) (`self.PaternCount`))))
  (`self.PaternAction`))

(event `self.ReceiveTick`
  (params (DeltaSeconds :type "Float (single-precision)"))
  ;[1 1 1] Event Tick
  (set `self.deltasec` DeltaSeconds))

(event `DoAction`
  ;[1 0 0] Enemy Attack
  (if (`self.hasspawned`)
    (switch `int` (`self.PaternCount`)
      (:`0`
        ;;[1 1 1] PHASE 2
        (if (and (not (`self.isAttacking`)) (> (`self.CurrentHealth`) 0.0))
          (set `self.isAttacking` true)
          (`self.SetEnemyAttack` (select `int` (`KismetMathLibrary.RandomIntegerInRange` 0 2) :`0` "NewEnumerator3" :`1` "NewEnumerator4" :`2` "NewEnumerator5" :!type "/Game/Blueprints/EN_Attacks Enum") true)))
      (:`1`
        ;;[1 1 1] PHASE 2
        (if (and (not (`self.isAttacking`)) (> (`self.CurrentHealth`) 0.0))
          (set `self.isAttacking` true)
          (`self.SetEnemyAttack` (select `int` (`KismetMathLibrary.RandomIntegerInRange` 0 2) :`0` "NewEnumerator0" :`1` "NewEnumerator1" :`2` "NewEnumerator2" :!type "/Game/Blueprints/EN_Attacks Enum") true))))))

(event `CameraShake`
  (params (Scale :type "Float (single-precision)"))
  (`MatineeCameraShake.StartMatineeCameraShake` (`GameplayStatics.GetPlayerCameraManager` 0) "/Game/Blueprints/BP_CameraShakeEnemy.BP_CameraShakeEnemy_C" Scale))

(event `PlayAnimationMontage`
  (params (Animation :type "AnimSequenceBase Object Reference"))
  ;[1 0.3465 0] Play Animation Shortcut
  (bind _returnvalue (`AnimInstance.PlaySlotAnimationAsDynamicMontage` (`SkeletalMeshComponent.GetAnimInstance` (`self.Mesh`)) Animation "DefaultSlot" 0.25 0.25 1.0 1 -1.0 0.0))
  (`KismetSystemLibrary.Delay` (`AnimationAsset.GetPlayLength` _returnvalue)))

(event `SpawnDamageAreaOnLocation`
  (params (Location :type "Vector Structure") (Radius :type "Float (double-precision)") (Damage :type "Float (double-precision)") (Parable :type Boolean :default true))
  ;[0 0.05878 1] Spawn Damage At Location
  (bind _outactors (`KismetSystemLibrary.SphereOverlapActors` Location Radius (`|MakeArray` "ObjectTypeQuery3" :!type "EObjectTypeQuery Enum") null (`|MakeArray` self :!type "Actor Object Reference")))
  (for _array_element _outactors
    (message `/Game/Blueprints/IT_Damage.DamageTarget` _array_element self (`self.ActorLocation`) Damage Parable)))

(event `SetEnemyAttack`
  (params (Attack :type "/Game/Blueprints/EN_Attacks Enum" :default "NewEnumerator0") (`LookAt?` :type Boolean))
  ;[0.5818 0.1701 1] Attack Action
  (`MovementComponent.StopMovementImmediately` (`self.CharacterMovement`))
  (if `LookAt?`
    (set `self.TargetPosition` (`self.K2_GetActorLocation` (`self.Player`)))
    (set `self.ActorLocation` (`self.K2_GetActorLocation`))
    (`TimelineComponent.SetPlayRate` (`self.TM_SetRotation`) 5.0)
    (bind (_direction _alpha) (`Timeline|TM_SetRotation` :!via `PlayFromStart`)
      (:`Update`
        (bind (_returnvalue_roll _returnvalue_pitch _returnvalue_yaw) (`KismetMathLibrary.BreakRotator` (`KismetMathLibrary.RLerp` (`self.K2_GetActorRotation`) (`KismetMathLibrary.FindLookAtRotation` (`self.ActorLocation`) (`self.TargetPosition`)) _alpha true)))
        (`self.K2_SetActorRotation` (`KismetMathLibrary.MakeRotator` 0.0 0.0 _returnvalue_yaw)))
      (:`Finished`
        (if (not (`self.isDead`)) :!label _label
          (switch `/Game/Blueprints/EN_Attacks` Attack
            (:`NewEnumerator3`
              (`self.Attack/ Kick Ground` :!label _label_2))
            (:`NewEnumerator4`
              (goto _label_2))
            (:`NewEnumerator5`
              (`self.Attack/ Charge`))
            (:`NewEnumerator0`
              (`self.Attack/Pantheon`))
            (:`NewEnumerator1`
              (if (`self.isPiloning`)
                (`self.SetEnemyAttack` (select `bool` (`KismetMathLibrary.RandomBool`) :`false` "NewEnumerator0" :`true` "NewEnumerator2" :!type "/Game/Blueprints/EN_Attacks Enum") true)
                (else
                  (`self.Attack/Pillar`))))
            (:`NewEnumerator2`
              (`self.Attack/Toupis`))))))
    (else
      (goto _label))))

(event `Attack/Pillar`
  ;[0.5818 0.1701 1] Attack Action
  ;;[0.06607 1 0.6206] Patern 1 / Marteau + Pylone
  (`self.PlayAnimationMontage` "/Game/3d/Cha/Titan/TitanColonnes_de_flammes.TitanColonnes_de_flammes"))

(event `HammerHitNotification`
  (bind (_returnvalue_x _returnvalue_y) (`KismetMathLibrary.BreakVector` (+ (`self.K2_GetActorLocation`) (* (`self.GetActorForwardVector`) 1000.0))))
  ;[0.5818 0.1701 1] Attack Action
  ;;[0.06607 1 0.6206] Patern 1 / Marteau + Pylone
  (set `self.isPiloning` true)
  (bind _returnvalue (`KismetSystemLibrary.K2_SetTimerDelegate` (delegate `SpawnPilier`) 0.7 true))
  (set `self.PilierHandle` _returnvalue)
  (`self.SpawnDamageAreaOnLocation` (`KismetMathLibrary.MakeVector` _returnvalue_x _returnvalue_y) 250.0 40.0)
  (`NiagaraFunctionLibrary.SpawnSystemAtLocation` "/Game/VFX/_Shared/NS_Boss_SmashGround.NS_Boss_SmashGround" (`KismetMathLibrary.MakeVector` _returnvalue_x _returnvalue_y))
  (`GameplayStatics.SpawnSound2D` "/Game/Audio/SFX/SFX_BossJumpImpact.SFX_BossJumpImpact" 1.0 1.0 0.0 null)
  (`self.CameraShake` 1.0)
  (bind _returnvalue_2 (`AnimInstance.PlaySlotAnimationAsDynamicMontage` (`SkeletalMeshComponent.GetAnimInstance` (`self.Mesh`)) "/Game/3d/Cha/Titan/TitanColonnes_de_flammesBack.TitanColonnes_de_flammesBack" "DefaultSlot" 0.25 0.25 1.0 1 -1.0 0.0))
  (`|ExecutionSequence`
    (:`then_0`
      (`KismetSystemLibrary.RetriggerableDelay` 10.0)
      (set `self.isPiloning` false)
      (`KismetSystemLibrary.K2_ClearAndInvalidateTimerHandle` (`self.PilierHandle`)))
    (:`then_1`
      (`KismetSystemLibrary.RetriggerableDelay` (- (`AnimationAsset.GetPlayLength` _returnvalue_2) 0.5))
      (set `self.isAttacking` false))))

(event `SpawnPilier`
  (bind (_returnvalue_x _returnvalue_y) (`KismetMathLibrary.BreakVector` (`SceneComponent.K2_GetComponentLocation` (`/Game/Blueprints/BP_Player.pillar_loc` (`self.Player`)))))
  ;[0.5818 0.1701 1] Attack Action
  ;;[0.06607 1 0.6206] Patern 1 / Marteau + Pylone
  (bind _returnvalue (`|SpawnActorFromClass` "/Game/Blueprints/BP_BossTotem.BP_BossTotem_C" (`KismetMathLibrary.MakeTransform` (`KismetMathLibrary.MakeVector` _returnvalue_x _returnvalue_y)) "Undefined" "OverrideRootScale" null null))
  (message `/Game/Blueprints/IT_Damage.DamageTarget` _returnvalue self (`self.K2_GetActorLocation`) 25.0 true)
  (`KismetSystemLibrary.Delay` 0.4)
  (`self.CameraShake` 1.0))

(event `Attack/Pantheon`
  (bind _returnvalue_location (`KismetMathLibrary.BreakTransform` (`self.GetTransform`)))
  ;[0.5818 0.1701 1] Attack Action
  ;;[0.4349 1 0.3233] Patern 2 / Saut + Atterissage
  (set `self.ignoreDamage` true)
  (bind _returnvalue (`AnimInstance.PlaySlotAnimationAsDynamicMontage` (`SkeletalMeshComponent.GetAnimInstance` (`self.Mesh`)) "/Game/3d/Cha/Titan/TitanPantheon.TitanPantheon" "DefaultSlot" 0.0 0.2 1.3 1 -1.0 0.0))
  (`GameplayStatics.PlaySoundAtLocation` "/Game/Audio/SFX/jumpststart.jumpststart" _returnvalue_location (struct) 1.0 1.0 0.0 null null null null)
  (`|ExecutionSequence`
    (:`then_0`
      (`KismetSystemLibrary.Delay` (+ (`AnimationAsset.GetPlayLength` _returnvalue) (`KismetMathLibrary.RandomFloatInRange` 0.0 1.0)))
      (set `self.isAttacking` false))
    (:`then_1`
      (`KismetSystemLibrary.Delay` 0.35)
      (`PrimitiveComponent.SetCastShadow` (`self.Mesh`) false))))

(event `PantheonHitNotification`
  (bind (_returnvalue_x _returnvalue_y) (`KismetMathLibrary.BreakVector` (`self.K2_GetActorLocation`)))
  ;[0.5818 0.1701 1] Attack Action
  ;;[0.4349 1 0.3233] Patern 2 / Saut + Atterissage
  (`self.SpawnDamageAreaOnLocation` (`KismetMathLibrary.MakeVector` _returnvalue_x _returnvalue_y) 900.0 70.0)
  (`NiagaraFunctionLibrary.SpawnSystemAtLocation` "/Game/VFX/_Shared/NS_Boss_JumpImpact.NS_Boss_JumpImpact" (`KismetMathLibrary.MakeVector` _returnvalue_x _returnvalue_y))
  (`GameplayStatics.SpawnSound2D` "/Game/Audio/SFX/SFX_BossJumpImpact.SFX_BossJumpImpact" 1.0 1.0 0.0 null)
  (`self.CameraShake` 3.0)
  (`PrimitiveComponent.SetCastShadow` (`self.Mesh`) true)
  (set `self.ignoreDamage` false))

(event `PantheonMoveToPlayerLocation`
  (bind (_returnvalue_x _returnvalue_y) (`KismetMathLibrary.BreakVector` (`self.K2_GetActorLocation`)))
  (bind (_returnvalue_x_2 _returnvalue_y_2) (`KismetMathLibrary.BreakVector` (`SceneComponent.K2_GetComponentLocation` (`/Game/Blueprints/BP_Player.jump_loc` (`self.Player`)))))
  ;[0.5818 0.1701 1] Attack Action
  ;;[0.4349 1 0.3233] Patern 2 / Saut + Atterissage
  (`self.K2_SetActorLocation` (`KismetMathLibrary.MakeVector` _returnvalue_x_2 _returnvalue_y_2 460.0))
  (`KismetSystemLibrary.Delay` 0.5)
  (`NiagaraFunctionLibrary.SpawnSystemAtLocation` "/Game/VFX/_Shared/NS_Boss_JumpZone.NS_Boss_JumpZone" (`KismetMathLibrary.MakeVector` _returnvalue_x _returnvalue_y)))

(event `Attack/Toupis`
  (bind _returnvalue_location (`KismetMathLibrary.BreakTransform` (`self.GetTransform`)))
  (bind (_returnvalue_location_2 _returnvalue_rotation _returnvalue_scale) (`KismetMathLibrary.BreakTransform` (`self.GetTransform`)))
  (bind _tornado (`self.Tornado`))
  (bind _capsulecomponent (`self.CapsuleComponent`))
  (bind (_returnvalue_roll _returnvalue_pitch _returnvalue_yaw) (`KismetMathLibrary.BreakRotator` (`SceneComponent.K2_GetComponentRotation` _capsulecomponent)))
  (bind _returnvalue_location_3 (`KismetMathLibrary.BreakTransform` (`self.GetTransform` (`|GetArrayItem` (`self.targetpoint`) (`self.currentpoint`)))))
  ;[0.5818 0.1701 1] Attack Action
  ;;[1 0.771 0.02762] Patern 3 / Toupis + Boule de feu
  (bind _returnvalue (`AnimInstance.PlaySlotAnimationAsDynamicMontage` (`SkeletalMeshComponent.GetAnimInstance` (`self.Mesh`)) "/Game/3d/Cha/Titan/TitanStart_Rotate.TitanStart_Rotate" "DefaultSlot" 0.25 0.1 1.5 1 -1.0 0.0))
  (`|ExecutionSequence`
    (:`then_0`
      (bind (_direction _newtrack_0) (`Timeline|Timeline_0` :!via `PlayFromStart`)
        (:`Update`
          (set `CameraComponent.FieldOfView` (`KismetMathLibrary.Lerp` 65.0 100.0 _newtrack_0) (`/Game/Blueprints/BP_Player.TopDownCamera` (`self.Player`)))
          (`KismetSystemLibrary.Delay` (- (`AnimationAsset.GetPlayLength` _returnvalue) 0.6))
          (bind _asbpa_titan (cast `/Game/Blueprints/BPA_Titan` (`SkeletalMeshComponent.GetAnimInstance` (`self.Mesh`))))
          (set `/Game/Blueprints/BPA_Titan.isRotating` true _asbpa_titan)
          (bind _returnvalue_2 (`KismetSystemLibrary.K2_SetTimerDelegate` (delegate `Shoot`) 0.03 true))
          (set `self.ToupisHandle` _returnvalue_2)
          (bind _returnvalue_3 (`NiagaraFunctionLibrary.SpawnSystemAttached` "/Game/VFX/_Shared/NS_Boss_FireTornado.NS_Boss_FireTornado" (`self.CapsuleComponent`) "None" (`SceneComponent.K2_GetComponentLocation` (`self.Mesh`)) (struct) "KeepWorldPosition"))
          (`PrimitiveComponent.SetTranslucentSortPriority` _returnvalue_3 10)
          (`ActorComponent.Activate` (`self.NS_Boss_HammerTrail`) false)
          (bind _output_get (set `self.Tornado` _returnvalue_3))
          (set `self.ToupisHandle` (struct))
          (bind (_direction_2 _alpha) (`Timeline|TM_Spining` :!via `PlayFromStart`)
            (:`Update`
              (`SceneComponent.K2_AddWorldRotation` _capsulecomponent (`KismetMathLibrary.MakeRotator` 0.0 0.0 (* _alpha (* 1400.0 (`self.deltasec`)))) false false)
              (`SceneComponent.K2_SetWorldRotation` :`self` _output_get)
              (`|ExecutionSequence`
                (:`then_0`
                  (if (> (`TimelineComponent.GetPlaybackPosition` (`self.TM_Spining`)) 9.0)
                    (`KismetSystemLibrary.K2_ClearAndInvalidateTimerHandle` (`self.ToupisHandle`))))
                (:`then_1`
                  (if (>= _returnvalue_yaw 150.0)
                    (`/Engine/EditorBlueprintResources/StandardMacros.DoOnce` false :!label _label_3
                      (:`Completed`
                        (`GameplayStatics.PlaySoundAtLocation` "/Game/Audio/Whoosh-Sound-Effect-HD-No-Copyright.Whoosh-Sound-Effect-HD-No-Copyright" _returnvalue_location (struct) 1.0 1.0 0.0 null null null null)))
                    (else
                      (goto _label_3 :!via `Reset`))))))
            (:`Finished`
              (`KismetSystemLibrary.K2_ClearAndInvalidateTimerHandle` (`self.ToupisHandle`))
              (bind _asbpa_titan_2 (cast `/Game/Blueprints/BPA_Titan` (`SkeletalMeshComponent.GetAnimInstance` (`self.Mesh`))))
              (`/Engine/EditorBlueprintResources/StandardMacros.IsValid` _tornado
                (:`Is Valid`
                  (`ActorComponent.Deactivate` _tornado)
                  (`ActorComponent.Deactivate` (`self.NS_Boss_HammerTrail`))
                  (set `/Game/Blueprints/BPA_Titan.isRotating` false _asbpa_titan_2)
                  (bind _returnvalue_4 (`AnimInstance.PlaySlotAnimationAsDynamicMontage` (`SkeletalMeshComponent.GetAnimInstance` (`self.Mesh`)) "/Game/3d/Cha/Titan/Titan_Idle_Anim.Titan_Idle_Anim" "DefaultSlot" 0.5 0.01 1.0 1 -1.0 0.0))
                  (bind (_direction_3 _newtrack_0_2) (`Timeline|Timeline_1` :!via `PlayFromStart`)
                    (:`Update`
                      (set `CameraComponent.FieldOfView` (`KismetMathLibrary.Lerp` 100.0 65.0 _newtrack_0_2) (`/Game/Blueprints/BP_Player.TopDownCamera` (`self.Player`)))
                      (`KismetSystemLibrary.Delay` (+ (`AnimationAsset.GetPlayLength` _returnvalue_4) (`KismetMathLibrary.RandomFloatInRange` 0.0 1.0)))
                      (set `self.isAttacking` false)
                      (`self.Reset/Toupis`))))))))))
    (:`then_1`
      (`KismetSystemLibrary.Delay` 2.0)
      (`/Engine/EditorBlueprintResources/StandardMacros.Do N` 3 :!label _label_4
        (:`Exit`
          (`|ExecutionSequence`
            (:`then_0`
              (while (== (`self.currentpoint`) (`self.lastpoint`))
                (set `self.currentpoint` (`KismetMathLibrary.RandomIntegerInRange` 0 3)))
              (set `self.kl` _returnvalue_location_3)
              (bind _output_get_2 (set `self.Nigg` _returnvalue_location_2))
              (bind (_direction_4 _newtrack_0_3) (`Timeline|Timeline_2` :!via `PlayFromStart`)
                (:`Update`
                  (bind (_returnvalue_x _returnvalue_y) (`KismetMathLibrary.BreakVector` (`KismetMathLibrary.VLerp` _output_get_2 (`self.kl`) _newtrack_0_3)))
                  (`self.K2_SetActorTransform` (`KismetMathLibrary.MakeTransform` (`KismetMathLibrary.MakeVector` _returnvalue_x _returnvalue_y (.z (.location (`self.GetTransform`)))) _returnvalue_rotation _returnvalue_scale))
                  (set `self.lastpoint` (`self.currentpoint`)))))
            (:`then_1`
              (`KismetSystemLibrary.RetriggerableDelay` 3.0)
              (goto _label_4))))))))

(event `Shoot`
  (bind _returnvalue (`SceneComponent.K2_GetComponentToWorld` (`self.CapsuleComponent`)))
  ;[0.5818 0.1701 1] Attack Action
  ;;[1 0.771 0.02762] Patern 3 / Toupis + Boule de feu
  (`self.SpawnDamageAreaOnLocation` (`self.K2_GetActorLocation`) 300.0 8.0)
  (if (> (`TimelineComponent.GetPlaybackPosition` (`self.TM_Spining`)) 1.5)
    (bind _output_get (set `self.savedtick` (+ (`self.savedtick`) 50.0)))
    (bind _returnvalue_2 (`|SpawnActorFromClass` "/Game/Blueprints/BP_BossProjectile.BP_BossProjectile_C" (`KismetMathLibrary.MakeTransform` (`KismetMathLibrary.MakeVector` (.x (.location _returnvalue)) (.y (.location _returnvalue)) 100.0) (`KismetMathLibrary.MakeRotator` (.roll (.rotation _returnvalue)) (.pitch (.rotation _returnvalue)) _output_get)) "Undefined" "OverrideRootScale" null null))
    (`/Engine/EditorBlueprintResources/StandardMacros.IsValid` _returnvalue_2
      (:`Is Valid`
        (message `/Game/Blueprints/IT_Damage.DamageTarget` _returnvalue_2 self (`self.K2_GetActorLocation`) 25.0 true)))))

(event `Reset/Toupis`
  ;[0.5818 0.1701 1] Attack Action
  ;;[1 0.771 0.02762] Patern 3 / Toupis + Boule de feu
  (goto _label_4 :!via `Reset`))

(event `DestroyAllParticles`
  (bind _tornado (`self.Tornado`))
  ;[0.5818 0.1701 1] Attack Action
  ;;[1 0.771 0.02762] Patern 3 / Toupis + Boule de feu
  (`/Engine/EditorBlueprintResources/StandardMacros.IsValid` _tornado
    (:`Is Valid`
      (`ActorComponent.K2_DestroyComponent` _tornado))))

(event `Attack/ Kick Ground`
  (bind _returnvalue (`SceneComponent.K2_GetComponentLocation` (`self.Mesh`)))
  ;[0.5818 0.1701 1] Attack Action
  ;;[1 0.2552 0.849] Patern 6 / Kick Ground
  (`AnimInstance.PlaySlotAnimationAsDynamicMontage` (`SkeletalMeshComponent.GetAnimInstance` (`self.Mesh`)) "/Game/3d/Cha/Titan/TitanCrush.TitanCrush" "DefaultSlot" 0.25 0.0 1.0 1 -1.0 0.0)
  (`KismetSystemLibrary.Delay` 1.1)
  (`|ExecutionSequence`
    (:`then_0`
      (`self.SpawnDamageAreaOnLocation` _returnvalue 500.0 25.0)
      (`NiagaraFunctionLibrary.SpawnSystemAtLocation` "/Game/VFX/_Shared/NS_Boss_KickGroundWave.NS_Boss_KickGroundWave" _returnvalue)
      (`GameplayStatics.SpawnSoundAtLocation` "/Game/Audio/SFX/SFX_BossJumpImpact.SFX_BossJumpImpact" _returnvalue (struct) 1.0 1.0 0.0 null null)
      (`KismetSystemLibrary.Delay` 2.0)
      (set `self.isAttacking` false))
    (:`then_1`
      (if (not (`/Game/Blueprints/BP_Player.attackDeflected` (`self.Player`)))
        (bind _returnvalue_2 (`KismetSystemLibrary.K2_SetTimerDelegate` (delegate `SpawnKickWave`) 0.05 true))
        (bind (_direction _alpha) (`Timeline|TM_KickGround` :!via `PlayFromStart`)
          (:`Update`
            (set `self.kickWaveRadius` _alpha))
          (:`Finished`
            (`KismetSystemLibrary.K2_ClearAndInvalidateTimerHandle` _returnvalue_2)))))))

(event `Attack/ Charge`
  ;[0.5818 0.1701 1] Attack Action
  ;;[1 0.5459 0.2491] Patern 4 / Charge
  (bind _returnvalue (`AnimInstance.PlaySlotAnimationAsDynamicMontage` (`SkeletalMeshComponent.GetAnimInstance` (`self.Mesh`)) "/Game/3d/Cha/Titan/TitanRush_Start.TitanRush_Start" "DefaultSlot" 0.25 0.0 1.0 1 -1.0 0.0))
  (`KismetSystemLibrary.Delay` (`AnimationAsset.GetPlayLength` _returnvalue))
  (set `self.isCharging` true)
  (set `self.ignoreDamage` true)
  (`AnimInstance.PlaySlotAnimationAsDynamicMontage` (`SkeletalMeshComponent.GetAnimInstance` (`self.Mesh`)) "/Game/3d/Cha/Titan/TitanRush_Run.TitanRush_Run" "DefaultSlot" 0.0 0.25 1.0 1000 -1.0 0.0)
  (bind (_direction _alpha) (`Timeline|TM_Charge` :!via `PlayFromStart` :!label _label_5)
    (:`Update`
      (`SceneComponent.K2_AddLocalOffset` (`self.CapsuleComponent`) (`KismetMathLibrary.MakeVector` (* _alpha (* 1400.0 (`self.deltasec`)))) false false))))

(event `self.CapsuleComponent.OnComponentBeginOverlap`
  (params (OverlappedComponent :type "PrimitiveComponent Object Reference") (OtherActor :type "Actor Object Reference") (OtherComp :type "PrimitiveComponent Object Reference") (OtherBodyIndex :type Integer) (bFromSweep :type Boolean) (SweepResult :type "HitResult Structure (by ref)"))
  (bind _returnvalue (`SceneComponent.K2_GetComponentLocation` (`self.CapsuleComponent`)))
  ;[0.5818 0.1701 1] Attack Action
  ;;[1 0.5459 0.2491] Patern 4 / Charge
  (bind _asbp_player (cast `/Game/Blueprints/BP_Player` OtherActor)
    (:`then`
      (if (`self.isCharging`)
        (message `/Game/Blueprints/IT_Damage.DamageTarget` _asbp_player self (0.0 0.0 0.0) 50.0 false)))
    (:`CastFailed`
      (if (and (`self.ActorHasTag` OtherActor "Wall") (`self.isCharging`))
        (`NiagaraFunctionLibrary.SpawnSystemAtLocation` "/Game/VFX/_Shared/NS_Boss_SmashGround.NS_Boss_SmashGround" _returnvalue)
        (`GameplayStatics.SpawnSoundAtLocation` "/Game/Audio/SFX/SFX_BossJumpImpact.SFX_BossJumpImpact" _returnvalue (struct) 1.0 1.0 0.0 null null)
        (set `self.isAttacking` false)
        (set `self.isCharging` true)
        (set `self.ignoreDamage` false)
        (`AnimInstance.PlaySlotAnimationAsDynamicMontage` (`SkeletalMeshComponent.GetAnimInstance` (`self.Mesh`)) "/Game/3d/Cha/Titan/TitanRush_Stop.TitanRush_Stop" "DefaultSlot" 0.25 0.25 1.0 1 -1.0 0.0)
        (goto _label_5 :!via `Stop`)))))

(event `SpawnKickWave`
  ;[0.5818 0.1701 1] Attack Action
  ;;[1 0.2552 0.849] Patern 6 / Kick Ground
  (`self.SpawnDamageAreaOnLocation` (`SceneComponent.K2_GetComponentLocation` (`self.Mesh`)) (`self.kickWaveRadius`) 10.0 false))

(fn `UserConstructionScript`)