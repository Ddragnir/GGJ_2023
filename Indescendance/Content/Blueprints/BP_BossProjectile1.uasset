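; Boss projectile actor that damages the player on overlap and turns to face the player as it exists.
; The DamageTarget event stores the initiator, damage value and Parable, which the sphere overlap forwards to BP_Player via DamageTargetMessage before destroying the actor.
; Overlapping a "Wall"-tagged actor spawns a fire-hit Niagara effect and also destroys it.
; BeginPlay caches BP_Player actors, and Tick rotates the root toward the first one.
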(event `/Game/Blueprints/IT_Damage.DamageTarget`
  (params (FromActor :type "Actor Object Reference") (FromLocation :type "Vector Structure") (DamageValue :type "Float (double-precision)") (Parable :type Boolean))
  (set `self.EnemyInitiator` FromActor)
  (set `self.DamageValue` DamageValue)
  (set `self.Parable` Parable))

(event `self.Sphere.OnComponentBeginOverlap`
  (params (OverlappedComponent :type "PrimitiveComponent Object Reference") (OtherActor :type "Actor Object Reference") (OtherComp :type "PrimitiveComponent Object Reference") (OtherBodyIndex :type Integer) (bFromSweep :type Boolean) (SweepResult :type "HitResult Structure (by ref)"))
  (bind _asbp_player (cast `/Game/Blueprints/BP_Player` OtherActor)
    (:`then`
      (message `/Game/Blueprints/IT_Damage.DamageTarget` _asbp_player (`self.EnemyInitiator`) (`self.K2_GetActorLocation`) (`self.DamageValue`) (`self.Parable`))
      (`self.K2_DestroyActor` :!label _label))
    (:`CastFailed`
      (if (`self.ActorHasTag` OtherActor "Wall")
        (`NiagaraFunctionLibrary.SpawnSystemAtLocation` "/Game/VFX/_Shared/NS_Boss_FireHit.NS_Boss_FireHit" (`self.K2_GetActorLocation`))
        (goto _label)))))

(event `self.ReceiveTick`
  (params (DeltaSeconds :type "Float (single-precision)"))
  (bind _defaultsceneroot (`self.DefaultSceneRoot`))
  (bind _returnvalue_location (`KismetMathLibrary.BreakTransform` (`SceneComponent.K2_GetComponentToWorld` _defaultsceneroot)))
  (bind _returnvalue_location_2 (`KismetMathLibrary.BreakTransform` (`self.GetTransform` (`|GetArrayItem` (stale `self.ReceiveBeginPlay` _outactors)))))
  (`SceneComponent.K2_SetWorldRotation` _defaultsceneroot (`KismetMathLibrary.FindLookAtRotation` _returnvalue_location _returnvalue_location_2) false false))

(event `self.ReceiveBeginPlay`
  (bind _outactors (`GameplayStatics.GetAllActorsOfClass` "/Game/Blueprints/BP_Player.BP_Player_C")))

(fn `UserConstructionScript`)