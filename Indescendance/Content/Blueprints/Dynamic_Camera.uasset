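; Dynamic camera actor that takes over the view when the player overlaps its start trigger and blends back at its end trigger.
; While it is the view target, Tick runs one of two modes.
; Stationary mode turns the camera to face the player.
; Otherwise it repositions the spring arm with VInterpTo, using a one-time captured offset and a per-axis TrackPlayer mask to choose which axes follow the player.
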(event `self.StartCamera.OnComponentBeginOverlap`
  (params (OverlappedComponent :type "PrimitiveComponent Object Reference") (OtherActor :type "Actor Object Reference") (OtherComp :type "PrimitiveComponent Object Reference") (OtherBodyIndex :type Integer) (bFromSweep :type Boolean) (SweepResult :type "HitResult Structure (by ref)"))
  (cast `/Game/Blueprints/BP_Player` OtherActor)
  (`PlayerController.SetViewTargetWithBlend` (`GameplayStatics.GetPlayerController` 0) self (`self.blend_Time`) "VTBlend_Linear" 0.0 false)
  (`/Engine/EditorBlueprintResources/StandardMacros.DoOnce` false
    (:`Completed`
      (set `self.offset` (- (`self.K2_GetActorLocation` (`GameplayStatics.GetPlayerCharacter` 0)) (`SceneComponent.K2_GetComponentLocation` (`self.SpringArm`)))))))

(event `self.EndCamera.OnComponentBeginOverlap`
  (params (OverlappedComponent :type "PrimitiveComponent Object Reference") (OtherActor :type "Actor Object Reference") (OtherComp :type "PrimitiveComponent Object Reference") (OtherBodyIndex :type Integer) (bFromSweep :type Boolean) (SweepResult :type "HitResult Structure (by ref)"))
  (bind _asbp_player (cast `/Game/Blueprints/BP_Player` OtherActor))
  (`PlayerController.SetViewTargetWithBlend` (`GameplayStatics.GetPlayerController` 0) _asbp_player (`self.blend_Time`) "VTBlend_Linear" 0.0 false))

(event `self.ReceiveTick`
  (params (DeltaSeconds :type "Float (single-precision)"))
  (if (== (`Controller.GetViewTarget` (`GameplayStatics.GetPlayerController` 0)) self)
    (if (`self.isStationary`)
      (bind _rotation (`self.trackPlayerRotation` DeltaSeconds))
      (`SceneComponent.K2_SetWorldRotation` (`self.Camera`) _rotation false false)
      (else
        (bind _vectoroutput (`self.trackPlayerMovement` DeltaSeconds))
        (`SceneComponent.K2_SetWorldLocation` (`self.SpringArm`) _vectoroutput false false)))))

(fn `trackPlayerMovement`
  (params (DeltaTime :type "Float (double-precision)"))
  (returns (VectorOutput :type "Vector Structure"))
  (bind _trackplayer (`self.trackPlayer`))
  (bind _returnvalue (- (`self.K2_GetActorLocation`) (`self.offset`)))
  (return (`KismetMathLibrary.VInterpTo` _returnvalue (+ (* (`self.K2_GetActorLocation` (`GameplayStatics.GetPlayerCharacter` 0)) _trackplayer) (* _returnvalue (- (1.0 1.0 1.0) _trackplayer))) DeltaTime)))

(fn `trackPlayerRotation`
  (params (Delta :type "Float (double-precision)"))
  (returns (Rotation :type "Rotator Structure"))
  (return (`KismetMathLibrary.FindLookAtRotation` (`SceneComponent.K2_GetComponentLocation` (`self.Camera`)) (`self.K2_GetActorLocation` (`GameplayStatics.GetPlayerCharacter` 0)))))

(fn `UserConstructionScript`)