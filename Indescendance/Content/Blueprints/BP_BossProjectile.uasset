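; BP_BossProjectile is a projectile, named for bosses, that delivers damage to the player on overlap.
; Its DamageTarget event stores the initiating actor, damage value and Parable setting.
; When its sphere overlaps a BP_Player, it forwards those values and its own location through a DamageTarget message, then destroys itself.
; Overlaps with other actors are ignored.
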(event `/Game/Blueprints/IT_Damage.DamageTarget`
  (params (FromActor :type "Actor Object Reference") (FromLocation :type "Vector Structure") (DamageValue :type "Float (double-precision)") (Parable :type Boolean))
  (set `self.EnemyInitiator` FromActor)
  (set `self.DamageValue` DamageValue)
  (set `self.Parable` Parable))

(event `self.Sphere.OnComponentBeginOverlap`
  (params (OverlappedComponent :type "PrimitiveComponent Object Reference") (OtherActor :type "Actor Object Reference") (OtherComp :type "PrimitiveComponent Object Reference") (OtherBodyIndex :type Integer) (bFromSweep :type Boolean) (SweepResult :type "HitResult Structure (by ref)"))
  (bind _asbp_player (cast `/Game/Blueprints/BP_Player` OtherActor))
  (message `/Game/Blueprints/IT_Damage.DamageTarget` _asbp_player (`self.EnemyInitiator`) (`self.K2_GetActorLocation`) (`self.DamageValue`) (`self.Parable`))
  (`self.K2_DestroyActor`))

(fn `UserConstructionScript`)