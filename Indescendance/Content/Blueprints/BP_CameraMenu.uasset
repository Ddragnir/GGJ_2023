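; BP_CameraMenu drives the main menu, creating the WG_Menu widget on BeginPlay and showing the mouse cursor.
; Start removes the menu, blends the view to BP_Player over a cubic transition, then possesses it and calls InitPlayer once the blend ends.
; Quit exits the game.
; An unconnected branch holds a level-sequence intro with PlayIntro that would rejoin the same blend.
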(event `self.ReceiveBeginPlay`
  (bind _returnvalue (`GameplayStatics.GetPlayerController` 0))
  (set `PlayerController.bShowMouseCursor` true _returnvalue)
  (bind _returnvalue_2 (`|CreateWidget` "/Game/Blueprints/WG_Menu.WG_Menu_C" _returnvalue))
  (bind _output_get (set `self.WGMenu` _returnvalue_2))
  (`UserWidget.AddToViewport` _output_get 0))

(event `CommencerButton Pressed`
  (bind _returnvalue (`GameplayStatics.GetPlayerController` 0))
  (bind _returnvalue_2 (`GameplayStatics.GetActorOfClass` "/Game/Blueprints/BP_Player.BP_Player_C"))
  (`Widget.RemoveFromParent` (`self.WGMenu`))
  (`PlayerController.SetViewTargetWithBlend` _returnvalue _returnvalue_2 2.0 "VTBlend_Cubic" 1.0 false)
  (`KismetSystemLibrary.Delay` 2.0)
  (`Controller.Possess` _returnvalue _returnvalue_2)
  (`/Game/Blueprints/BP_Player.InitPlayer` _returnvalue_2))

(event `QuitterButtonPressed`
  (`KismetSystemLibrary.QuitGame` null "Quit"))

(fn `UserConstructionScript`)